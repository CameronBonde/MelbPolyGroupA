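; AI bear character that wanders the NavMesh and attacks what it detects.
; A state switch, entered on BeginPlay and re-run via UpdateState, alternates wandering with a distance check choosing super hug when close or knee attack otherwise.
; Tick box-traces along a vector scaled from actor location, not facing, to set the target.
; Taking damage triggers a random move, death animation and surprise grenade spawn before wandering resumes.
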(event Custom|Update%20state
  (switch Utilities|FlowControl|Switch|SwitchonMurilo_actions (Variables|Default|GetState)
    (:NewEnumerator2
      ;[1 1 1] knee Attack
      (AI|AIMoveTo (Class|PawnMovementComponent|GetPawnOwner (Variables|Character|GetCharacterMovement)) "0, 0, 0" (Variables|Default|GetLastseem) 5.0 false
        (:OnSuccess
          (Components|Animation|PlayAnimation (Variables|Default|GetEnemy_Bear) "/Game/InfinityBladeAdversaries/Enemy/Enemy_Bear/Enemy_Bear_Animations/ExoGame_Bears_Drop_Down.ExoGame_Bears_Drop_Down" false)
          (Game|Damage|ApplyDamage 0 0.0 0 0)
          (Development|PrintString "knee attach")
          (Utilities|FlowControl|Delay 1.0)
          (Variables|Default|SetState "NewEnumerator4")
          (CallFunction|UpdateState))))
    (:NewEnumerator1
      ;[1 1 1] SuperHug
      (AI|AIMoveTo (Class|PawnMovementComponent|GetPawnOwner (Variables|Character|GetCharacterMovement)) "0.000000,0.000000,0.000000" (Variables|Default|GetLastseem) 5.0 false
        (:OnSuccess
          (Components|Animation|PlayAnimation (Variables|Default|GetEnemy_Bear) "/Game/InfinityBladeAdversaries/Enemy/Enemy_Bear/Enemy_Bear_Animations/ExoGame_Bears_Attack_Melee_C.ExoGame_Bears_Attack_Melee_C" false)
          (Game|Damage|ApplyDamage 0 5e+01 0 0)
          (Development|PrintString "hugggggg")
          (Utilities|FlowControl|Delay 1.0)
          (Variables|Default|SetState "NewEnumerator4")
          (CallFunction|UpdateState))))
    (:NewEnumerator0
      ;[1 1 1] Receiving damage
      (Components|Animation|PlayAnimation (Variables|Default|GetEnemy_Bear) "/Game/InfinityBladeAdversaries/Enemy/Enemy_Bear/Enemy_Bear_Animations/ExoGame_Bears_Attack_Death_2.ExoGame_Bears_Attack_Death_2" false)
      (Utilities|FlowControl|Delay 1.3)
      (Development|PrintString "Surpise")
      ;[1 1 1] Grenade left
      (Game|SpawnActorfromClass "/Game/People/MuriloMachado/BluePrints/Granade.Granade_C" (Transformation|GetWorldTransform (Variables|Default|Getgrenadespawpoint)) "Undefined" 0 0)
      (Components|Animation|PlayAnimation (Variables|Default|GetEnemy_Bear) "/Game/InfinityBladeAdversaries/Enemy/Enemy_Bear/Enemy_Bear_Animations/ExoGame_Bears_Walk.ExoGame_Bears_Walk" false)
      ;[1 1 1] Exit
      (Utilities|FlowControl|Delay (Variables|Default|GetStart))
      (AI|Navigation|SimpleMovetoLocation (Pawn|GetController) (AI|Navigation|GetRandomReachablePointinRadius (Transformation|GetActorLocation) 3e+04))
      (Variables|Default|SetState "NewEnumerator4")
      (CallFunction|UpdateState))
    (:NewEnumerator4
      ;[1 1 1] Wondering
      (Utilities|FlowControl|Delay (Variables|Default|GetStart))
      (Components|Animation|PlayAnimation (Variables|Default|GetEnemy_Bear) "/Game/InfinityBladeAdversaries/Enemy/Enemy_Bear/Enemy_Bear_Animations/ExoGame_Bears_Walk.ExoGame_Bears_Walk" true)
      (AI|Navigation|SimpleMovetoLocation (Pawn|GetController) (AI|Navigation|GetRandomReachablePointinRadius (Transformation|GetActorLocation) 1.1e+04))
      (Utilities|FlowControl|Delay 5.0)
      (CallFunction|CheckDistance))))

(event Custom|Check%20Distance
  ;[1 1 1] check distance
  (if (Utilities|IsValid (Variables|Default|GetLastseem))
    ;[1 1 1] Attack decision
    (if (<= (Transformation|GetDistanceTo self (Variables|Default|GetLastseem)) (Variables|Default|Getdistance))
      (Variables|Default|SetState "NewEnumerator1")
      (CallFunction|UpdateState)
      (else
        (Variables|Default|SetState "NewEnumerator2")
        (CallFunction|UpdateState)))
    (else
      (CallFunction|UpdateState))))

(event Custom|CheckEnemy
  ;[1 1 1] Looking for enemies
  (bind (_outhit _returnvalue) (Collision|BoxTraceByChannel (Transformation|GetActorLocation) (+ (Transformation|GetActorLocation) (* (Transformation|GetActorLocation) 1e+01)) "100.000000,400.000000,100.000000" (Transformation|GetActorRotation) "TraceTypeQuery1" false 0 "None"))
  (if _returnvalue
    (Variables|Default|SetLastseem (.hitactor _outhit))))

(event EventTick
  (params (DeltaSeconds :type Float%20%28single-precision%29))
  ;[1 1 1] Main
  (CallFunction|CheckEnemy))

(event EventBeginPlay
  (switch Utilities|FlowControl|Switch|SwitchonMurilo_actions (Variables|Default|GetState)
    (:NewEnumerator2
      ;[1 1 1] knee Attack
      (AI|AIMoveTo (Class|PawnMovementComponent|GetPawnOwner (Variables|Character|GetCharacterMovement)) "0, 0, 0" (Variables|Default|GetLastseem) 5.0 false
        (:OnSuccess
          (Components|Animation|PlayAnimation (Variables|Default|GetEnemy_Bear) "/Game/InfinityBladeAdversaries/Enemy/Enemy_Bear/Enemy_Bear_Animations/ExoGame_Bears_Drop_Down.ExoGame_Bears_Drop_Down" false)
          (Game|Damage|ApplyDamage 0 0.0 0 0)
          (Development|PrintString "knee attach")
          (Utilities|FlowControl|Delay 1.0)
          (Variables|Default|SetState "NewEnumerator4")
          (CallFunction|UpdateState))))
    (:NewEnumerator1
      ;[1 1 1] SuperHug
      (AI|AIMoveTo (Class|PawnMovementComponent|GetPawnOwner (Variables|Character|GetCharacterMovement)) "0.000000,0.000000,0.000000" (Variables|Default|GetLastseem) 5.0 false
        (:OnSuccess
          (Components|Animation|PlayAnimation (Variables|Default|GetEnemy_Bear) "/Game/InfinityBladeAdversaries/Enemy/Enemy_Bear/Enemy_Bear_Animations/ExoGame_Bears_Attack_Melee_C.ExoGame_Bears_Attack_Melee_C" false)
          (Game|Damage|ApplyDamage 0 5e+01 0 0)
          (Development|PrintString "hugggggg")
          (Utilities|FlowControl|Delay 1.0)
          (Variables|Default|SetState "NewEnumerator4")
          (CallFunction|UpdateState))))
    (:NewEnumerator0
      ;[1 1 1] Receiving damage
      (Components|Animation|PlayAnimation (Variables|Default|GetEnemy_Bear) "/Game/InfinityBladeAdversaries/Enemy/Enemy_Bear/Enemy_Bear_Animations/ExoGame_Bears_Attack_Death_2.ExoGame_Bears_Attack_Death_2" false)
      (Utilities|FlowControl|Delay 1.3)
      (Development|PrintString "Surpise")
      ;[1 1 1] Grenade left
      (Game|SpawnActorfromClass "/Game/People/MuriloMachado/BluePrints/Granade.Granade_C" (Transformation|GetWorldTransform (Variables|Default|Getgrenadespawpoint)) "Undefined" 0 0)
      (Components|Animation|PlayAnimation (Variables|Default|GetEnemy_Bear) "/Game/InfinityBladeAdversaries/Enemy/Enemy_Bear/Enemy_Bear_Animations/ExoGame_Bears_Walk.ExoGame_Bears_Walk" false)
      ;[1 1 1] Exit
      (Utilities|FlowControl|Delay (Variables|Default|GetStart))
      (AI|Navigation|SimpleMovetoLocation (Pawn|GetController) (AI|Navigation|GetRandomReachablePointinRadius (Transformation|GetActorLocation) 3e+04))
      (Variables|Default|SetState "NewEnumerator4")
      (CallFunction|UpdateState))
    (:NewEnumerator4
      ;[1 1 1] Wondering
      (Utilities|FlowControl|Delay (Variables|Default|GetStart))
      (Components|Animation|PlayAnimation (Variables|Default|GetEnemy_Bear) "/Game/InfinityBladeAdversaries/Enemy/Enemy_Bear/Enemy_Bear_Animations/ExoGame_Bears_Walk.ExoGame_Bears_Walk" true)
      (AI|Navigation|SimpleMovetoLocation (Pawn|GetController) (AI|Navigation|GetRandomReachablePointinRadius (Transformation|GetActorLocation) 1.1e+04))
      (Utilities|FlowControl|Delay 5.0)
      (CallFunction|CheckDistance))))

(event Game|Damage|EventAnyDamage
  (params (Damage :type Float%20%28single-precision%29) (DamageType :type Damage%20Type%20Object%20Reference) (InstigatedBy :type Controller%20Object%20Reference) (DamageCauser :type Actor%20Object%20Reference))
  ;[1 1 1] Receiving damage
  (AI|Navigation|SimpleMovetoLocation (Pawn|GetController) (AI|Navigation|GetRandomReachablePointinRadius (Transformation|GetActorLocation) 1.5e+04))
  (Components|Animation|PlayAnimation (Variables|Default|GetEnemy_Bear) "/Game/InfinityBladeAdversaries/Enemy/Enemy_Bear/Enemy_Bear_Animations/ExoGame_Bears_Attack_Death_2.ExoGame_Bears_Attack_Death_2" false)
  (Utilities|FlowControl|Delay 1.3)
  (Development|PrintString "Surpise")
  ;[1 1 1] Grenade left
  (Game|SpawnActorfromClass "/Game/People/MuriloMachado/BluePrints/Granade.Granade_C" (Transformation|GetWorldTransform (Variables|Default|Getgrenadespawpoint)) "Undefined" 0 0)
  (Components|Animation|PlayAnimation (Variables|Default|GetEnemy_Bear) "/Game/InfinityBladeAdversaries/Enemy/Enemy_Bear/Enemy_Bear_Animations/ExoGame_Bears_Walk.ExoGame_Bears_Walk" false)
  ;[1 1 1] Exit
  (Utilities|FlowControl|Delay (Variables|Default|GetStart))
  (AI|Navigation|SimpleMovetoLocation (Pawn|GetController) (AI|Navigation|GetRandomReachablePointinRadius (Transformation|GetActorLocation) 3e+04))
  (Variables|Default|SetState "NewEnumerator4")
  (CallFunction|UpdateState))

(fn ConstructionScript)