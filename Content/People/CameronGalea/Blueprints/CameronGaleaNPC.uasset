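; A Gruntling NPC that picks behavior from a state enum: wander, move to buddy, idle, kamikaze or S.O.S.
; Each state drives text, animation, movement or spawning another NPC, re-entered through UpdateState on Tick.
; A forward box trace each tick records the last seen actor; after wandering, seeing its own class leads to Idle, anything else to Kamikaze.
; Damage sets an angry flag that these graphs never read.
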(event OnComponentBeginOverlap(CapsuleComponent)
  (params (OtherActor :type Actor%20Object%20Reference) (OtherComp :type Primitive%20Component%20Object%20Reference) (OtherBodyIndex :type Integer) (bFromSweep :type Boolean) (SweepResult :type Hit%20Result%20Structure%20%28by%20ref%29))
  ;[1 1 1] Senses
)

(event Custom|Update%20State
  ;[1 1 1] Random Condition
  (switch Utilities|FlowControl|Switch|SwitchonCameronGaleaStates (Variables|Default|GetCurrentState)
    (:NewEnumerator0
      ;[1 1 1] Wandering
      (Utilities|FlowControl|Delay (Math|Random|RandomFloatinRange 1.0 5.0))
      (Rendering|Components|TextRender|SetText (Variables|Default|GetTextRender) (Variables|Default|GetWanderingText))
      (Components|Animation|PlayAnimation (Variables|Character|GetMesh) "/Game/InfinityBladeAdversaries/Enemy/Enemy_Gruntling_Avalanche/Enemy_Gruntling_Avalanche_Animation/ExoGame_Gruntling_Run.ExoGame_Gruntling_Run" true)
      (AI|AIMoveTo (Class|PawnMovementComponent|GetPawnOwner (Variables|Character|GetCharacterMovement)) (AI|Navigation|GetRandomReachablePointinRadius (Transformation|GetActorLocation) 1e+05) 0 5.0 false
        (:OnSuccess
          (Audio|Components|Audio|Stop (Variables|Character|GetMesh))
          (Utilities|IsValid (Variables|Default|GetLast%20seen%20actor)
            (:Is%20Valid
              (Utilities|Casting|CastToCameronGaleaNPC (Variables|Default|GetLast%20seen%20actor)
                (:then
                  (Variables|Default|SetCurrentState "NewEnumerator8"))
                (:CastFailed
                  (Variables|Default|SetCurrentState "NewEnumerator9")))
              (CallFunction|UpdateState))))))
    (:NewEnumerator1
      ;[1 1 1] Move to buddy
      (Utilities|FlowControl|Delay (Math|Random|RandomFloatinRange 1.0 5.0))
      (Rendering|Components|TextRender|SetText (Variables|Default|GetTextRender) (Variables|Default|GetBuddyText))
      (Character|Jump)
      (Utilities|FlowControl|Delay 1.0)
      (Character|Jump)
      (AI|Navigation|SimpleMovetoActor (Pawn|GetController) (Variables|Default|GetBuddy))
      (CallFunction|UpdateState))
    (:NewEnumerator9
      (Components|Animation|PlayAnimation (Variables|Character|GetMesh) "/Game/InfinityBladeAdversaries/Enemy/Enemy_Gruntling_Avalanche/Enemy_Gruntling_Avalanche_Animation/ExoGame_Gruntling_On_Fire.ExoGame_Gruntling_On_Fire" false))
    (:NewEnumerator8
      ;[1 1 1] Idle
      (Rendering|Components|TextRender|SetText (Variables|Default|GetTextRender) (Variables|Default|GetIdleText))
      (Components|Animation|PlayAnimation (Variables|Character|GetMesh) "/Game/InfinityBladeAdversaries/Enemy/Enemy_Gruntling_Avalanche/Enemy_Gruntling_Avalanche_Animation/ExoGame_Gruntling_React_Stunned_Idle.ExoGame_Gruntling_React_Stunned_Idle" true)
      (Utilities|FlowControl|Delay (Math|Random|RandomFloatinRange 1.0 5.0))
      (CallFunction|UpdateState))
    (:NewEnumerator7
      ;[1 1 1] S.O.S
      (Utilities|FlowControl|Delay 2.0)
      (Rendering|Components|TextRender|SetText (Variables|Default|GetTextRender) (Variables|Default|GetS.O.SText))
      (AI|SpawnAIFromClass "CameronGaleaNPC_C" 0 (Transformation|GetActorLocation) "0, 0, 0" false))))

(event Custom|CheckSight
  ;[1 1 1] Senses
  (bind (_outhit _returnvalue) (Collision|BoxTraceByChannel (Transformation|GetActorLocation) (+ (Transformation|GetActorLocation) (* (Transformation|GetActorForwardVector) 1e+04)) "0,200.000000, 0" (Transformation|GetActorRotation) "TraceTypeQuery2" false 0 "ForOneFrame"))
  (if _returnvalue
    (Variables|Default|SetLast%20seen%20actor (.hitactor _outhit))))

(event EventTick
  (params (DeltaSeconds :type Float%20%28single-precision%29))
  (CallFunction|UpdateState)
  (CallFunction|CheckSight))

(event Game|Damage|EventAnyDamage
  (params (Damage :type Float%20%28single-precision%29) (DamageType :type Damage%20Type%20Object%20Reference) (InstigatedBy :type Controller%20Object%20Reference) (DamageCauser :type Actor%20Object%20Reference))
  (Variables|Default|SetAmAngry true))

(event EventBeginPlay
  ;[1 1 1] Random Condition
  (switch Utilities|FlowControl|Switch|SwitchonCameronGaleaStates (Variables|Default|GetCurrentState)
    (:NewEnumerator0
      ;[1 1 1] Wandering
      (Utilities|FlowControl|Delay (Math|Random|RandomFloatinRange 1.0 5.0))
      (Rendering|Components|TextRender|SetText (Variables|Default|GetTextRender) (Variables|Default|GetWanderingText))
      (Components|Animation|PlayAnimation (Variables|Character|GetMesh) "/Game/InfinityBladeAdversaries/Enemy/Enemy_Gruntling_Avalanche/Enemy_Gruntling_Avalanche_Animation/ExoGame_Gruntling_Run.ExoGame_Gruntling_Run" true)
      (AI|AIMoveTo (Class|PawnMovementComponent|GetPawnOwner (Variables|Character|GetCharacterMovement)) (AI|Navigation|GetRandomReachablePointinRadius (Transformation|GetActorLocation) 1e+05) 0 5.0 false
        (:OnSuccess
          (Audio|Components|Audio|Stop (Variables|Character|GetMesh))
          (Utilities|IsValid (Variables|Default|GetLast%20seen%20actor)
            (:Is%20Valid
              (Utilities|Casting|CastToCameronGaleaNPC (Variables|Default|GetLast%20seen%20actor)
                (:then
                  (Variables|Default|SetCurrentState "NewEnumerator8"))
                (:CastFailed
                  (Variables|Default|SetCurrentState "NewEnumerator9")))
              (CallFunction|UpdateState))))))
    (:NewEnumerator1
      ;[1 1 1] Move to buddy
      (Utilities|FlowControl|Delay (Math|Random|RandomFloatinRange 1.0 5.0))
      (Rendering|Components|TextRender|SetText (Variables|Default|GetTextRender) (Variables|Default|GetBuddyText))
      (Character|Jump)
      (Utilities|FlowControl|Delay 1.0)
      (Character|Jump)
      (AI|Navigation|SimpleMovetoActor (Pawn|GetController) (Variables|Default|GetBuddy))
      (CallFunction|UpdateState))
    (:NewEnumerator9
      (Components|Animation|PlayAnimation (Variables|Character|GetMesh) "/Game/InfinityBladeAdversaries/Enemy/Enemy_Gruntling_Avalanche/Enemy_Gruntling_Avalanche_Animation/ExoGame_Gruntling_On_Fire.ExoGame_Gruntling_On_Fire" false))
    (:NewEnumerator8
      ;[1 1 1] Idle
      (Rendering|Components|TextRender|SetText (Variables|Default|GetTextRender) (Variables|Default|GetIdleText))
      (Components|Animation|PlayAnimation (Variables|Character|GetMesh) "/Game/InfinityBladeAdversaries/Enemy/Enemy_Gruntling_Avalanche/Enemy_Gruntling_Avalanche_Animation/ExoGame_Gruntling_React_Stunned_Idle.ExoGame_Gruntling_React_Stunned_Idle" true)
      (Utilities|FlowControl|Delay (Math|Random|RandomFloatinRange 1.0 5.0))
      (CallFunction|UpdateState))
    (:NewEnumerator7
      ;[1 1 1] S.O.S
      (Utilities|FlowControl|Delay 2.0)
      (Rendering|Components|TextRender|SetText (Variables|Default|GetTextRender) (Variables|Default|GetS.O.SText))
      (AI|SpawnAIFromClass "CameronGaleaNPC_C" 0 (Transformation|GetActorLocation) "0, 0, 0" false))))

(fn ConstructionScript)