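; CameronBondeNPC is an NPC whose enum state machine covers wandering, approaching a buddy, spawning an AIGuy (Merge), idling, damage reaction and a line-of-sight attack.
; UpdateState re-enters the state switch from BeginPlay.
; Tick box-traces ahead to record LastSeenActor.
; The attack timeline turns toward that actor, aborting if line traces lose it, otherwise applying damage; every state change here, including on damage, sets Wander.
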(event OnComponentEndOverlap(SightSphere)
  (params (OtherActor :type Actor%20Object%20Reference) (OtherComp :type Primitive%20Component%20Object%20Reference) (OtherBodyIndex :type Integer))
  ;[1 1 1] Senses
)

(event OnComponentBeginOverlap(SightSphere)
  (params (OtherActor :type Actor%20Object%20Reference) (OtherComp :type Primitive%20Component%20Object%20Reference) (OtherBodyIndex :type Integer) (bFromSweep :type Boolean) (SweepResult :type Hit%20Result%20Structure%20%28by%20ref%29))
  ;[1 1 1] Senses
)

(event OnHearNoise(PawnSensing)
  (params (Instigator :type Pawn%20Object%20Reference) (Location :type Vector%20%28by%20ref%29 :default "0, 0, 0") (Volume :type Float%20%28single-precision%29))
  ;[1 1 1] Senses
  (Variables|Default|SetLast%20Heard%20Pawn Instigator))

(event Custom|CheckSight
  ;[1 1 1] Senses
  (bind (_outhit _returnvalue) (Collision|BoxTraceByChannel (Transformation|GetActorLocation) (+ (Transformation|GetActorLocation) (* (Transformation|GetActorForwardVector) 1e+03)) "0.000000,200.000000,0.000000" (Transformation|GetActorRotation) "TraceTypeQuery2" false 0 "None"))
  (if _returnvalue
    (Variables|Default|SetLast%20Seen%20Actor (.hitactor _outhit))))

(event Custom|UpdateState
  ;[1 1 1] State machine
  (switch Utilities|FlowControl|Switch|SwitchonCameronBondeStates (Variables|Default|GetCurrentState)
    (:NewEnumerator0
      ;[1 1 1] Wander
      (Components|Animation|PlayAnimation (Variables|Character|GetMesh) 0 true)
      (AI|AIMoveTo (Class|PawnMovementComponent|GetPawnOwner (Variables|Character|GetCharacterMovement)) (AI|Navigation|GetRandomReachablePointinRadius (Transformation|GetActorLocation) 1e+04) 0 5.0 false
        (:OnSuccess
          (Components|Animation|PlayAnimation (Variables|Character|GetMesh) 0 true)
          (Utilities|FlowControl|Delay 2.0)
          (Utilities|IsValid (Variables|Default|GetLast%20Seen%20Actor) ; Did I see ANYONE?
            (:Is%20Valid
              (Variables|Default|SetCurrentState "NewEnumerator0")
              (CallFunction|UpdateState))
            (:Is%20Not%20Valid
              (Variables|Default|SetCurrentState "NewEnumerator0")
              (CallFunction|UpdateState))))))
    (:NewEnumerator1
      ;[1 1 1] Move to buddy. Happy!
      (Rendering|Components|TextRender|SetText (Variables|Default|GetTextRender) (Variables|Default|GetWooMessage))
      (Character|Jump)
      (Utilities|FlowControl|Delay 1.0)
      (Character|Jump)
      (AI|Navigation|SimpleMovetoActor (Pawn|GetController) (Variables|Default|GetBuddy)))
    (:NewEnumerator2
      ;[1 1 1] Hover
      (Development|PrintString "hOVER"))
    (:NewEnumerator3
      ;[1 1 1] Merge
      (Class|PawnNoiseEmitterComponent|MakeNoise (Variables|Default|GetPawnNoiseEmitter) 0 1.0 (Transformation|GetActorLocation))
      (Components|Animation|PlayAnimation (Variables|Character|GetMesh) 0 false)
      (Utilities|FlowControl|Delay 0.5)
      (Game|SpawnActorfromClass "/Game/People/CameronBonde/Blueprints/AIGuy.AIGuy_C" (Transformation|GetWorldTransform (Variables|Default|GetIn%20front%20spawn%20point)) "Undefined" 0 0)
      (Utilities|FlowControl|Delay 4.0)
      (Variables|Default|SetCurrentState "NewEnumerator0")
      (CallFunction|UpdateState))
    (:NewEnumerator4
      ;[1 1 1] Idle
      (Utilities|FlowControl|Delay (Math|Random|RandomFloatinRange 1.0 3.0))
      (Variables|Default|SetCurrentState "NewEnumerator0"))
    (:NewEnumerator5
      ;[1 1 1] Line of sight attack
      (Components|Animation|PlayAnimation (Variables|Character|GetMesh) 0 false)
      (Utilities|FlowControl|Delay 0.75)
      (Variables|/Script/Engine.SkeletalMeshComponent|SetbPauseAnims (Variables|Character|GetMesh) true)
      (Timeline|Check%20LOS PlayFromStart
        (:Update
          (|Rotatetotarget)
          (bind _outhit (Collision|LineTraceByChannel (Transformation|GetActorLocation) (Transformation|GetActorLocation (Variables|Default|GetLast%20Seen%20Actor)) "TraceTypeQuery1" false 0 "ForOneFrame"))
          ;[1 1 1] Target hid, so abort back to wandering
          (if (not (== (.hitactor _outhit) (Variables|Default|GetLast%20Seen%20Actor)))
            (Audio|Components|Audio|Stop (Variables|Default|GetCheck%20LOS))
            (Variables|Default|SetLast%20Seen%20Actor 0)
            (Variables|Default|SetCurrentState "NewEnumerator0")
            (CallFunction|UpdateState)))
        (:Finished
          (Game|Damage|ApplyDamage (Variables|Default|GetLast%20Seen%20Actor) 1e+02 0 self)
          (Variables|/Script/Engine.SkeletalMeshComponent|SetbPauseAnims (Variables|Character|GetMesh) false)
          (Utilities|FlowControl|Delay 1.0)
          (Variables|Default|SetCurrentState "NewEnumerator0")
          (CallFunction|UpdateState))))
    (:NewEnumerator6
      ;[1 1 1] Damaged
      (Components|Animation|PlayAnimation (Variables|Character|GetMesh) 0 false)
      (Utilities|FlowControl|Delay 2.0)
      (Variables|Default|SetCurrentState "NewEnumerator0")
      (CallFunction|UpdateState))))

(event EventBeginPlay
  ;[1 1 1] State machine
  (switch Utilities|FlowControl|Switch|SwitchonCameronBondeStates (Variables|Default|GetCurrentState)
    (:NewEnumerator0
      ;[1 1 1] Wander
      (Components|Animation|PlayAnimation (Variables|Character|GetMesh) 0 true)
      (AI|AIMoveTo (Class|PawnMovementComponent|GetPawnOwner (Variables|Character|GetCharacterMovement)) (AI|Navigation|GetRandomReachablePointinRadius (Transformation|GetActorLocation) 1e+04) 0 5.0 false
        (:OnSuccess
          (Components|Animation|PlayAnimation (Variables|Character|GetMesh) 0 true)
          (Utilities|FlowControl|Delay 2.0)
          (Utilities|IsValid (Variables|Default|GetLast%20Seen%20Actor) ; Did I see ANYONE?
            (:Is%20Valid
              (Variables|Default|SetCurrentState "NewEnumerator0")
              (CallFunction|UpdateState))
            (:Is%20Not%20Valid
              (Variables|Default|SetCurrentState "NewEnumerator0")
              (CallFunction|UpdateState))))))
    (:NewEnumerator1
      ;[1 1 1] Move to buddy. Happy!
      (Rendering|Components|TextRender|SetText (Variables|Default|GetTextRender) (Variables|Default|GetWooMessage))
      (Character|Jump)
      (Utilities|FlowControl|Delay 1.0)
      (Character|Jump)
      (AI|Navigation|SimpleMovetoActor (Pawn|GetController) (Variables|Default|GetBuddy)))
    (:NewEnumerator2
      ;[1 1 1] Hover
      (Development|PrintString "hOVER"))
    (:NewEnumerator3
      ;[1 1 1] Merge
      (Class|PawnNoiseEmitterComponent|MakeNoise (Variables|Default|GetPawnNoiseEmitter) 0 1.0 (Transformation|GetActorLocation))
      (Components|Animation|PlayAnimation (Variables|Character|GetMesh) 0 false)
      (Utilities|FlowControl|Delay 0.5)
      (Game|SpawnActorfromClass "/Game/People/CameronBonde/Blueprints/AIGuy.AIGuy_C" (Transformation|GetWorldTransform (Variables|Default|GetIn%20front%20spawn%20point)) "Undefined" 0 0)
      (Utilities|FlowControl|Delay 4.0)
      (Variables|Default|SetCurrentState "NewEnumerator0")
      (CallFunction|UpdateState))
    (:NewEnumerator4
      ;[1 1 1] Idle
      (Utilities|FlowControl|Delay (Math|Random|RandomFloatinRange 1.0 3.0))
      (Variables|Default|SetCurrentState "NewEnumerator0"))
    (:NewEnumerator5
      ;[1 1 1] Line of sight attack
      (Components|Animation|PlayAnimation (Variables|Character|GetMesh) 0 false)
      (Utilities|FlowControl|Delay 0.75)
      (Variables|/Script/Engine.SkeletalMeshComponent|SetbPauseAnims (Variables|Character|GetMesh) true)
      (Timeline|Check%20LOS PlayFromStart
        (:Update
          (|Rotatetotarget)
          (bind _outhit (Collision|LineTraceByChannel (Transformation|GetActorLocation) (Transformation|GetActorLocation (Variables|Default|GetLast%20Seen%20Actor)) "TraceTypeQuery1" false 0 "ForOneFrame"))
          ;[1 1 1] Target hid, so abort back to wandering
          (if (not (== (.hitactor _outhit) (Variables|Default|GetLast%20Seen%20Actor)))
            (Audio|Components|Audio|Stop (Variables|Default|GetCheck%20LOS))
            (Variables|Default|SetLast%20Seen%20Actor 0)
            (Variables|Default|SetCurrentState "NewEnumerator0")
            (CallFunction|UpdateState)))
        (:Finished
          (Game|Damage|ApplyDamage (Variables|Default|GetLast%20Seen%20Actor) 1e+02 0 self)
          (Variables|/Script/Engine.SkeletalMeshComponent|SetbPauseAnims (Variables|Character|GetMesh) false)
          (Utilities|FlowControl|Delay 1.0)
          (Variables|Default|SetCurrentState "NewEnumerator0")
          (CallFunction|UpdateState))))
    (:NewEnumerator6
      ;[1 1 1] Damaged
      (Components|Animation|PlayAnimation (Variables|Character|GetMesh) 0 false)
      (Utilities|FlowControl|Delay 2.0)
      (Variables|Default|SetCurrentState "NewEnumerator0")
      (CallFunction|UpdateState))))

(event EventTick
  (params (DeltaSeconds :type Float%20%28single-precision%29))
  ;[1 1 1] Main loop
  (CallFunction|CheckSight))

(event Game|Damage|EventAnyDamage
  (params (Damage :type Float%20%28single-precision%29) (DamageType :type Damage%20Type%20Object%20Reference) (InstigatedBy :type Controller%20Object%20Reference) (DamageCauser :type Actor%20Object%20Reference))
  ;[1 1 1] Senses
  (Variables|Default|SetEnemy DamageCauser)
  (Variables|Default|SetCurrentState "NewEnumerator0")
  (CallFunction|UpdateState))

(fn ConstructionScript)