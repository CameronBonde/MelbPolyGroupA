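; AI character Blueprint that runs a simple enum state machine: Heat Up Neighbours, Wander and Teleport.
; Heating up spins the actor on a timeline, then Wander walks to a random reachable point and, after a delay, may switch to Teleport.
; A per-tick forward box trace records LastSeenActor, which Teleport jumps to after spinning, before wandering again.
; Damage sets an AmAngry flag that the states never read.
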(event Custom|CheckSight
  ;[1 1 1] Senses and Memory
  ;;[1 1 1] Sight
  (bind (_outhit _returnvalue) (Collision|BoxTraceByChannel (Transformation|GetActorLocation) (+ (Transformation|GetActorLocation) (* (Transformation|GetActorForwardVector) 1e+03)) "0.000000,200.000000,0.000000" (Transformation|GetActorRotation) "TraceTypeQuery2" false 0 "ForOneFrame"))
  (if _returnvalue ; Did we hit anything?
    (Variables|Default|SetLast%20seen%20actor (.hitactor _outhit))))

(event Custom|Update%20state
  (switch Utilities|FlowControl|Switch|SwitchonAIGuyStates (Variables|Default|GetState)
    (:NewEnumerator0
      ;[1 1 1] Heat up neighbours
      ;;[1 1 1] Enter
      (Development|PrintString "Heating up neighbours start")
      ;;[1 1 1] Update
      (Timeline|Timeline_0 Play
        (:Update
          (Class|Actor|AddActorWorldRotation "0,10.000000, 0") ; Spin
        )
        (:Finished
          ;;[1 1 1] Exit
          (Variables|Default|SetState "NewEnumerator1")
          (CallFunction|UpdateState))))
    (:NewEnumerator1
      ;[1 1 1] Wander
      (Development|PrintString "Wander Enter")
      (AI|Navigation|SimpleMovetoLocation (Pawn|GetController) (AI|Navigation|GetRandomReachablePointinRadius (Transformation|GetActorLocation) 1e+04))
      (Utilities|FlowControl|Delay (Math|Random|RandomFloatinRange 5.0 1e+01))
      ;[1 1 1] Change  State to Teleport
      (if (!= (Variables|Default|GetLast%20seen%20actor) "AIGuy_C")
        (Variables|Default|SetState "NewEnumerator3")
        (CallFunction|UpdateState)))
    (:NewEnumerator3
      ;[1 1 1] Teleport
      (Development|PrintString "Teleport")
      (Utilities|FlowControl|Delay 2.0)
      (Timeline|Spin%20for%20a%20bit Play
        (:Update
          (Transformation|AddRelativeRotation (Variables|Collision|GetCapsuleComponent) "0,10.000000, 0" false false))
        (:Finished
          (Transformation|SetActorLocation (Transformation|GetActorLocation (Variables|Default|GetLast%20seen%20actor)) false false) ; Teleport
          (Variables|Default|SetState "NewEnumerator1")
          (CallFunction|UpdateState))))))

(event Game|Damage|EventAnyDamage
  (params (Damage :type Float%20%28single-precision%29) (DamageType :type Damage%20Type%20Object%20Reference) (InstigatedBy :type Controller%20Object%20Reference) (DamageCauser :type Actor%20Object%20Reference))
  ;[1 1 1] Senses and Memory
  ;;[1 1 1] Damage
  (Variables|Default|SetAmAngry true))

(event EventBeginPlay
  (switch Utilities|FlowControl|Switch|SwitchonAIGuyStates (Variables|Default|GetState)
    (:NewEnumerator0
      ;[1 1 1] Heat up neighbours
      ;;[1 1 1] Enter
      (Development|PrintString "Heating up neighbours start")
      ;;[1 1 1] Update
      (Timeline|Timeline_0 Play
        (:Update
          (Class|Actor|AddActorWorldRotation "0,10.000000, 0") ; Spin
        )
        (:Finished
          ;;[1 1 1] Exit
          (Variables|Default|SetState "NewEnumerator1")
          (CallFunction|UpdateState))))
    (:NewEnumerator1
      ;[1 1 1] Wander
      (Development|PrintString "Wander Enter")
      (AI|Navigation|SimpleMovetoLocation (Pawn|GetController) (AI|Navigation|GetRandomReachablePointinRadius (Transformation|GetActorLocation) 1e+04))
      (Utilities|FlowControl|Delay (Math|Random|RandomFloatinRange 5.0 1e+01))
      ;[1 1 1] Change  State to Teleport
      (if (!= (Variables|Default|GetLast%20seen%20actor) "AIGuy_C")
        (Variables|Default|SetState "NewEnumerator3")
        (CallFunction|UpdateState)))
    (:NewEnumerator3
      ;[1 1 1] Teleport
      (Development|PrintString "Teleport")
      (Utilities|FlowControl|Delay 2.0)
      (Timeline|Spin%20for%20a%20bit Play
        (:Update
          (Transformation|AddRelativeRotation (Variables|Collision|GetCapsuleComponent) "0,10.000000, 0" false false))
        (:Finished
          (Transformation|SetActorLocation (Transformation|GetActorLocation (Variables|Default|GetLast%20seen%20actor)) false false) ; Teleport
          (Variables|Default|SetState "NewEnumerator1")
          (CallFunction|UpdateState))))))

(event EventTick
  (params (DeltaSeconds :type Float%20%28single-precision%29))
  (CallFunction|CheckSight))

(fn ConstructionScript)