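; SmallCharacter is a jumping character that moves toward a Sphere_Blueprint actor it detects.
; From BeginPlay it loops every second, jumping and issuing SimpleMoveToActor toward the stored Thing; the random branch has no effect.
; Sightsphere overlaps enter the same chain midway, storing the overlapping actor as Thing and jumping again when it casts to Sphere_Blueprint.
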(event OnComponentBeginOverlap(sightsphere)
  (params (OtherActor :type Actor%20Object%20Reference) (OtherComp :type Primitive%20Component%20Object%20Reference) (OtherBodyIndex :type Integer) (bFromSweep :type Boolean) (SweepResult :type Hit%20Result%20Structure%20%28by%20ref%29))
  (bind _assphere_blueprint (Utilities|Casting|CastToSphere_Blueprint OtherActor :!label _label)
    (:then
      (Variables|Default|Setthing _assphere_blueprint)
      (Character|Jump))
    (:CastFailed
      _))
  (AI|Navigation|SimpleMovetoActor (Pawn|GetController) (Variables|Default|Getthing))
  (Utilities|FlowControl|Delay 1.0)
  (if (Math|Random|RandomBool)
    _
    (else
      _))
  (Character|Jump)
  (goto _label))

(event EventBeginPlay
  (if (Math|Random|RandomBool) :!label _label
    _
    (else
      _))
  (Character|Jump)
  (bind _assphere_blueprint (Utilities|Casting|CastToSphere_Blueprint (stale OnComponentBeginOverlap(sightsphere) OtherActor))
    (:then
      (Variables|Default|Setthing _assphere_blueprint)
      (Character|Jump))
    (:CastFailed
      _))
  (AI|Navigation|SimpleMovetoActor (Pawn|GetController) (Variables|Default|Getthing))
  (Utilities|FlowControl|Delay 1.0)
  (goto _label))

(fn ConstructionScript)