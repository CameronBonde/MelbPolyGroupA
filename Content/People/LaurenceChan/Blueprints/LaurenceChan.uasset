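; LaurenceChan is a spider AI character driven by an enum state machine that loops through BeginPlay and UpdateState.
; It alternates between wandering to random points and summoning an Egg at the last actor seen by a per-tick forward box trace.
; Guard and explode states exist, the latter chasing and applying radial damage, but nothing here switches into them.
; Damage only sets an anger flag, and cube hits make LaurenceChan actors jump.
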(event OnComponentHit(Cube1)
  (params (OtherActor :type Actor%20Object%20Reference) (OtherComp :type Primitive%20Component%20Object%20Reference) (NormalImpulse :type Vector :default "0, 0, 0") (Hit :type Hit%20Result%20Structure%20%28by%20ref%29))
  ;[1 1 1] OnHit Jump
  (bind _aslaurence_chan (Utilities|Casting|CastToLaurenceChan OtherActor))
  (Character|Jump _aslaurence_chan))

(event Custom|UpdateState
  (switch Utilities|FlowControl|Switch|SwitchonLaurenceChanStates (Variables|Default|GetCurrentState)
    (:NewEnumerator0
      ;[1 1 1] Wander
      (Components|Animation|PlayAnimation (Variables|Default|GetSkeletalMesh) "/Game/InfinityBladeAdversaries/Enemy/Enemy_Great_Spider/Enemy_SpiderGreater_Animation/ExoGame_Greater_Spider_Walk_Fwd.ExoGame_Greater_Spider_Walk_Fwd" true)
      (AI|Navigation|SimpleMovetoLocation (Pawn|GetController) (AI|Navigation|GetRandomReachablePointinRadius (Transformation|GetActorLocation) 1e+04))
      (Utilities|FlowControl|Delay (Math|Random|RandomFloatinRange 0.0 4.0))
      (Variables|Default|SetCurrentState "NewEnumerator1")
      (CallFunction|UpdateState))
    (:NewEnumerator1
      ;[1 1 1] Spawn Egg
      (Components|Animation|SetAnimation (Variables|Default|GetSkeletalMesh) 0)
      (Development|PrintString "egg")
      (Utilities|FlowControl|Delay 3.0)
      (Components|Animation|PlayAnimation (Variables|Default|GetSkeletalMesh) "/Game/InfinityBladeAdversaries/Enemy/Enemy_Great_Spider/Enemy_SpiderGreater_Animation/ExoGame_Greater_Spider_Cast_Summon.ExoGame_Greater_Spider_Cast_Summon" false)
      (Game|SpawnActorfromClass "/Game/People/LaurenceChan/Blueprints/Egg.Egg_C" (Math|Transform|MakeTransform (Transformation|GetActorLocation (Variables|Default|GetLast%20Seen%20Actor)) "0, 0, 0" "1,1,1") "AdjustIfPossibleButAlwaysSpawn" 0 0)
      (Variables|Default|SetCurrentState "NewEnumerator0")
      (CallFunction|UpdateState))
    (:NewEnumerator2
      ;[1 1 1] Guard Egg
      (Development|PrintString "guard")
      (Utilities|FlowControl|Delay 3.0)
      (CallFunction|UpdateState))
    (:NewEnumerator3
      ;[1 1 1] Explode on Death
      (if (!= (Variables|Default|GetLast%20Seen%20Actor) 0)
        (AI|Navigation|SimpleMovetoActor (Pawn|GetController) (Variables|Default|GetLast%20Seen%20Actor))
        (Utilities|FlowControl|Delay 3.0)
        (Effects|SpawnEmitterAttached 0 0 "None")
        (Game|Damage|ApplyRadialDamage 1e+04 (Transformation|GetWorldLocation (Variables|Default|GetCube1)) 5e+03 0 0 0 0 false "ECC_Visibility")
        (Development|PrintString "explode")
        (Variables|Default|SetCurrentState "NewEnumerator0")
        (CallFunction|UpdateState)))))

(event Custom|CheckSight
  ;[1 1 1] Senses
  (bind (_outhit _returnvalue) (Collision|BoxTraceByChannel (Transformation|GetActorLocation) (+ (Transformation|GetActorLocation) (* (Transformation|GetActorForwardVector) 1e+03)) "0,400.000000, 0" (Transformation|GetActorRotation) "TraceTypeQuery2" false 0 "ForOneFrame"))
  (if _returnvalue
    (Variables|Default|SetLast%20Seen%20Actor (.hitactor _outhit))))

(event EventBeginPlay
  (switch Utilities|FlowControl|Switch|SwitchonLaurenceChanStates (Variables|Default|GetCurrentState)
    (:NewEnumerator0
      ;[1 1 1] Wander
      (Components|Animation|PlayAnimation (Variables|Default|GetSkeletalMesh) "/Game/InfinityBladeAdversaries/Enemy/Enemy_Great_Spider/Enemy_SpiderGreater_Animation/ExoGame_Greater_Spider_Walk_Fwd.ExoGame_Greater_Spider_Walk_Fwd" true)
      (AI|Navigation|SimpleMovetoLocation (Pawn|GetController) (AI|Navigation|GetRandomReachablePointinRadius (Transformation|GetActorLocation) 1e+04))
      (Utilities|FlowControl|Delay (Math|Random|RandomFloatinRange 0.0 4.0))
      (Variables|Default|SetCurrentState "NewEnumerator1")
      (CallFunction|UpdateState))
    (:NewEnumerator1
      ;[1 1 1] Spawn Egg
      (Components|Animation|SetAnimation (Variables|Default|GetSkeletalMesh) 0)
      (Development|PrintString "egg")
      (Utilities|FlowControl|Delay 3.0)
      (Components|Animation|PlayAnimation (Variables|Default|GetSkeletalMesh) "/Game/InfinityBladeAdversaries/Enemy/Enemy_Great_Spider/Enemy_SpiderGreater_Animation/ExoGame_Greater_Spider_Cast_Summon.ExoGame_Greater_Spider_Cast_Summon" false)
      (Game|SpawnActorfromClass "/Game/People/LaurenceChan/Blueprints/Egg.Egg_C" (Math|Transform|MakeTransform (Transformation|GetActorLocation (Variables|Default|GetLast%20Seen%20Actor)) "0, 0, 0" "1,1,1") "AdjustIfPossibleButAlwaysSpawn" 0 0)
      (Variables|Default|SetCurrentState "NewEnumerator0")
      (CallFunction|UpdateState))
    (:NewEnumerator2
      ;[1 1 1] Guard Egg
      (Development|PrintString "guard")
      (Utilities|FlowControl|Delay 3.0)
      (CallFunction|UpdateState))
    (:NewEnumerator3
      ;[1 1 1] Explode on Death
      (if (!= (Variables|Default|GetLast%20Seen%20Actor) 0)
        (AI|Navigation|SimpleMovetoActor (Pawn|GetController) (Variables|Default|GetLast%20Seen%20Actor))
        (Utilities|FlowControl|Delay 3.0)
        (Effects|SpawnEmitterAttached 0 0 "None")
        (Game|Damage|ApplyRadialDamage 1e+04 (Transformation|GetWorldLocation (Variables|Default|GetCube1)) 5e+03 0 0 0 0 false "ECC_Visibility")
        (Development|PrintString "explode")
        (Variables|Default|SetCurrentState "NewEnumerator0")
        (CallFunction|UpdateState)))))

(event Game|Damage|EventAnyDamage
  (params (Damage :type Float%20%28single-precision%29) (DamageType :type Damage%20Type%20Object%20Reference) (InstigatedBy :type Controller%20Object%20Reference) (DamageCauser :type Actor%20Object%20Reference))
  ;[1 1 1] Senses
  (Variables|Default|SetIs%20Angry true)
  (Development|PrintString "Ouch"))

(event EventTick
  (params (DeltaSeconds :type Float%20%28single-precision%29))
  ;[1 1 1] EventTickUpdater
  (CallFunction|CheckSight))

(fn ConstructionScript)