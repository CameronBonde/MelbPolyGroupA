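; CharlotteAllingham2 is an AI bear actor with rough Avoid, Wander and Follow states.
; BeginPlay and Updatestate switch on CurentState: Wander loops random navmesh moves with timeline-driven idle and walk animations, while Avoid and Follow are mostly debug-print stubs.
; SightInFront line-traces forward, setting the differently spelled CurrentState to Follow on hitting its own class, otherwise Avoid.
; AnyDamage sets the idle animation.
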(event Custom|Update%20state
  (switch Utilities|FlowControl|Switch|SwitchonCharlotteAllinghamstates (Variables|Default|GetCurent%20state)
    (:NewEnumerator1
      ;[1 1 1] Avoid
      (Development|PrintString "Avoid")
      (Utilities|FlowControl|Delay 3.0))
    (:NewEnumerator0
      ;[1 1 1] Walking
      (AI|Navigation|SimpleMovetoLocation (Pawn|GetController) (AI|Navigation|GetRandomReachablePointinRadius (Transformation|GetActorLocation) 1e+03) :!label _label)
      (Utilities|FlowControl|Delay 4.0)
      (Timeline|Timeline_0 PlayFromStart
        (:Update
          (Components|Animation|PlayAnimation (Variables|Default|GetSkeletalMesh) "/Game/InfinityBladeAdversaries/Enemy/Enemy_Bear/Enemy_Bear_Animations/ExoGame_Bears_Idle.ExoGame_Bears_Idle" true))
        (:Finished
          (Components|Animation|PlayAnimation (Variables|Default|GetSkeletalMesh) "/Game/InfinityBladeAdversaries/Enemy/Enemy_Bear/Enemy_Bear_Animations/ExoGame_Bears_Walk.ExoGame_Bears_Walk" true)
          (goto _label))))
    (:NewEnumerator2
      ;[1 1 1] Follow
      (Development|PrintString "Follow")
      (Utilities|FlowControl|Delay 0.2)
      (Components|Animation|PlayAnimation (Variables|Default|GetSkeletalMesh) "/Game/InfinityBladeAdversaries/Enemy/Enemy_Bear/Enemy_Bear_Animations/ExoGame_Bears_Idle.ExoGame_Bears_Idle" false)
      (Audio|Components|Audio|Stop (Variables|Default|GetSkeletalMesh)))))

(event Custom|SightInFront
  ;[1 1 1] Sight
  (bind _outhit (Collision|LineTraceByChannel (Transformation|GetActorLocation) (+ (Transformation|GetActorLocation) (* (Transformation|GetActorForwardVector) 10000)) "TraceTypeQuery1" false 0 "ForOneFrame"))
  (Utilities|Casting|CastToCharlotteAllingham2 (.hitactor _outhit)
    (:then
      (Variables|Default|SetCurrent%20State "NewEnumerator2"))
    (:CastFailed
      (Variables|Default|SetCurrent%20State "NewEnumerator1"))))

(event Game|Damage|EventAnyDamage
  (params (Damage :type Float%20%28single-precision%29) (DamageType :type Damage%20Type%20Object%20Reference) (InstigatedBy :type Controller%20Object%20Reference) (DamageCauser :type Actor%20Object%20Reference))
  ;[1 1 1] Damage
  (Components|Animation|SetAnimation (Variables|Default|GetSkeletalMesh) "/Game/InfinityBladeAdversaries/Enemy/Enemy_Bear/Enemy_Bear_Animations/ExoGame_Bears_Idle.ExoGame_Bears_Idle"))

(event EventBeginPlay
  (switch Utilities|FlowControl|Switch|SwitchonCharlotteAllinghamstates (Variables|Default|GetCurent%20state)
    (:NewEnumerator1
      ;[1 1 1] Avoid
      (Development|PrintString "Avoid")
      (Utilities|FlowControl|Delay 3.0))
    (:NewEnumerator0
      ;[1 1 1] Walking
      (AI|Navigation|SimpleMovetoLocation (Pawn|GetController) (AI|Navigation|GetRandomReachablePointinRadius (Transformation|GetActorLocation) 1e+03) :!label _label)
      (Utilities|FlowControl|Delay 4.0)
      (Timeline|Timeline_0 PlayFromStart
        (:Update
          (Components|Animation|PlayAnimation (Variables|Default|GetSkeletalMesh) "/Game/InfinityBladeAdversaries/Enemy/Enemy_Bear/Enemy_Bear_Animations/ExoGame_Bears_Idle.ExoGame_Bears_Idle" true))
        (:Finished
          (Components|Animation|PlayAnimation (Variables|Default|GetSkeletalMesh) "/Game/InfinityBladeAdversaries/Enemy/Enemy_Bear/Enemy_Bear_Animations/ExoGame_Bears_Walk.ExoGame_Bears_Walk" true)
          (goto _label))))
    (:NewEnumerator2
      ;[1 1 1] Follow
      (Development|PrintString "Follow")
      (Utilities|FlowControl|Delay 0.2)
      (Components|Animation|PlayAnimation (Variables|Default|GetSkeletalMesh) "/Game/InfinityBladeAdversaries/Enemy/Enemy_Bear/Enemy_Bear_Animations/ExoGame_Bears_Idle.ExoGame_Bears_Idle" false)
      (Audio|Components|Audio|Stop (Variables|Default|GetSkeletalMesh)))))

(fn ConstructionScript)