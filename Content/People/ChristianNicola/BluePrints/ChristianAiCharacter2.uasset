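; AI greater-spider character that teleports in with a lightning effect, then wanders and melee-attacks actors it sees.
; A state switch re-entered through UpdateState drives random roaming with idle pauses, or chasing and damaging a target before wandering again.
; A forward box trace each Tick records the last seen actor, which becomes the enemy after a wander pause unless it is a ChristianAiCharacter.
; A Bomb Drop death state spawns an EggBomb, but its trigger is unconnected.
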(event Custom|CheckSight
  ;[1 1 1] Senses
  ;;[1 1 1] Sight
  (bind (_outhit _returnvalue) (Collision|BoxTraceByChannel (Transformation|GetActorLocation) (+ (Transformation|GetActorLocation) (* (Transformation|GetActorForwardVector) 1e+04)) "100.000000,400.000000,100.000000" (Transformation|GetActorRotation) "TraceTypeQuery1" false 0 "None"))
  (if _returnvalue
    (Variables|Default|SetLastSeenActor (.hitactor _outhit))))

(event Custom|UpdateState
  (bind _lastseenactor (Variables|Default|GetLastSeenActor))
  ;[1 1 1] Random Condition
  (switch Utilities|FlowControl|Switch|SwitchonChristianNicolaStates (Variables|Default|GetCurrent%20State)
    (:NewEnumerator0
      ;[1 1 1] Wander
      (Components|Animation|PlayAnimation (Variables|Default|GetSK_Greater_Spider) "/Game/InfinityBladeAdversaries/Enemy/Enemy_Great_Spider/Enemy_SpiderGreater_Animation/ExoGame_Greater_Spider_Walk_Fwd.ExoGame_Greater_Spider_Walk_Fwd" true)
      (AI|AIMoveTo (Class|PawnMovementComponent|GetPawnOwner (Variables|Character|GetCharacterMovement)) (AI|Navigation|GetRandomReachablePointinRadius (Transformation|GetActorLocation) 1e+04) 0 5.0 false
        (:OnSuccess
          (Components|Animation|PlayAnimation (Variables|Default|GetSK_Greater_Spider) "/Game/InfinityBladeAdversaries/Enemy/Enemy_Great_Spider/Enemy_SpiderGreater_Animation/ExoGame_Greater_Spider_Idle.ExoGame_Greater_Spider_Idle" true)
          (Utilities|FlowControl|Delay (Math|Random|RandomFloatinRange 1.0 1e+01))
          (Utilities|Casting|CastToChristianAiCharacter _lastseenactor
            (:then
              (CallFunction|UpdateState))
            (:CastFailed
              (Utilities|IsValid _lastseenactor
                (:Is%20Valid
                  (Variables|Default|SetEnemy _lastseenactor)
                  (Variables|Default|SetCurrent%20State "NewEnumerator3")
                  (CallFunction|UpdateState))))))))
    (:NewEnumerator3
      ;[1 1 1] Melee Attack
      (Utilities|IsValid (Variables|Default|GetEnemy)
        (:Is%20Valid
          (AI|AIMoveTo (Class|PawnMovementComponent|GetPawnOwner (Variables|Character|GetCharacterMovement)) "0, 0, 0" (Variables|Default|GetEnemy) 2.0 false
            (:OnSuccess
              (Components|Animation|PlayAnimation (Variables|Default|GetSK_Greater_Spider) "/Game/InfinityBladeAdversaries/Enemy/Enemy_Great_Spider/Enemy_SpiderGreater_Animation/ExoGame_Greater_Spider_Attack_Melee.ExoGame_Greater_Spider_Attack_Melee" false)
              (Game|Damage|ApplyDamage (Variables|Default|GetLastSeenActor) 1e+02 0 self)
              (Utilities|FlowControl|Delay 3.0)
              (Variables|Default|SetCurrent%20State "NewEnumerator0")
              (CallFunction|UpdateState))))
        (:Is%20Not%20Valid
          (Variables|Default|SetCurrent%20State "NewEnumerator0")
          (CallFunction|UpdateState))))
    (:NewEnumerator4
      ;[1 1 1] Bomb Drop
      (Development|PrintString "SCREECH!")
      (Components|Animation|PlayAnimation (Variables|Default|GetSK_Greater_Spider) "/Game/InfinityBladeAdversaries/Enemy/Enemy_Great_Spider/Enemy_SpiderGreater_Animation/ExoGame_Greater_Spider_Death.ExoGame_Greater_Spider_Death" false)
      (Utilities|FlowControl|Delay 2.0)
      (Audio|Components|Audio|Stop (Variables|Default|GetSK_Greater_Spider))
      (Effects|SpawnEmitterAttached "/Game/InfinityBladeEffects/Effects/FX_Ambient/Fog/P_ExitStair_Mist.P_ExitStair_Mist" (Variables|Default|GetParticleSystem) "None")
      (Game|SpawnActorfromClass "/Game/People/ChristianNicola/BluePrints/EggBomb.EggBomb_C" (Transformation|GetActorTransform) "Undefined" 0 0)
      (Utilities|FlowControl|Delay 5.0)
      (Actor|DestroyActor))))

(event Game|Damage|EventAnyDamage
  (params (Damage :type Float%20%28single-precision%29) (DamageType :type Damage%20Type%20Object%20Reference) (InstigatedBy :type Controller%20Object%20Reference) (DamageCauser :type Actor%20Object%20Reference))
  ;[1 1 1] Senses
  (Variables|Default|SetAggro true)
  (Variables|Default|SetEnemy InstigatedBy))

(event EventTick
  (params (DeltaSeconds :type Float%20%28single-precision%29))
  ;[1 1 1] EventTickUpdater
  (CallFunction|CheckSight))

(event EventBeginPlay
  (bind _lastseenactor (Variables|Default|GetLastSeenActor))
  ;[1 1 1] Character Spawn Animation
  (bind _returnvalue (Effects|SpawnEmitterAttached "/Game/InfinityBladeEffects/Effects/FX_Monsters/FX_Monster_Genno/P_Genno_Weapon_Lightning_01.P_Genno_Weapon_Lightning_01" (Variables|Default|GetParticleSystem) "None" "0, 0, 0" "0, 0, 0" "KeepRelativeOffset" false))
  (Components|Animation|PlayAnimation (Variables|Default|GetSK_Greater_Spider) "/Game/InfinityBladeAdversaries/Enemy/Enemy_Great_Spider/Enemy_SpiderGreater_Animation/ExoGame_Greater_Spider_Teleport.ExoGame_Greater_Spider_Teleport" false)
  (Timeline|Timeline_0 PlayFromStart
    (:Finished
      (Components|Activation|Deactivate _returnvalue)
      (Audio|Components|Audio|Stop (Variables|Default|GetSK_Greater_Spider))
      (Utilities|FlowControl|Delay 0.5)
      ;[1 1 1] Random Condition
      (switch Utilities|FlowControl|Switch|SwitchonChristianNicolaStates (Variables|Default|GetCurrent%20State)
        (:NewEnumerator0
          ;[1 1 1] Wander
          (Components|Animation|PlayAnimation (Variables|Default|GetSK_Greater_Spider) "/Game/InfinityBladeAdversaries/Enemy/Enemy_Great_Spider/Enemy_SpiderGreater_Animation/ExoGame_Greater_Spider_Walk_Fwd.ExoGame_Greater_Spider_Walk_Fwd" true)
          (AI|AIMoveTo (Class|PawnMovementComponent|GetPawnOwner (Variables|Character|GetCharacterMovement)) (AI|Navigation|GetRandomReachablePointinRadius (Transformation|GetActorLocation) 1e+04) 0 5.0 false
            (:OnSuccess
              (Components|Animation|PlayAnimation (Variables|Default|GetSK_Greater_Spider) "/Game/InfinityBladeAdversaries/Enemy/Enemy_Great_Spider/Enemy_SpiderGreater_Animation/ExoGame_Greater_Spider_Idle.ExoGame_Greater_Spider_Idle" true)
              (Utilities|FlowControl|Delay (Math|Random|RandomFloatinRange 1.0 1e+01))
              (Utilities|Casting|CastToChristianAiCharacter _lastseenactor
                (:then
                  (CallFunction|UpdateState))
                (:CastFailed
                  (Utilities|IsValid _lastseenactor
                    (:Is%20Valid
                      (Variables|Default|SetEnemy _lastseenactor)
                      (Variables|Default|SetCurrent%20State "NewEnumerator3")
                      (CallFunction|UpdateState))))))))
        (:NewEnumerator3
          ;[1 1 1] Melee Attack
          (Utilities|IsValid (Variables|Default|GetEnemy)
            (:Is%20Valid
              (AI|AIMoveTo (Class|PawnMovementComponent|GetPawnOwner (Variables|Character|GetCharacterMovement)) "0, 0, 0" (Variables|Default|GetEnemy) 2.0 false
                (:OnSuccess
                  (Components|Animation|PlayAnimation (Variables|Default|GetSK_Greater_Spider) "/Game/InfinityBladeAdversaries/Enemy/Enemy_Great_Spider/Enemy_SpiderGreater_Animation/ExoGame_Greater_Spider_Attack_Melee.ExoGame_Greater_Spider_Attack_Melee" false)
                  (Game|Damage|ApplyDamage (Variables|Default|GetLastSeenActor) 1e+02 0 self)
                  (Utilities|FlowControl|Delay 3.0)
                  (Variables|Default|SetCurrent%20State "NewEnumerator0")
                  (CallFunction|UpdateState))))
            (:Is%20Not%20Valid
              (Variables|Default|SetCurrent%20State "NewEnumerator0")
              (CallFunction|UpdateState))))
        (:NewEnumerator4
          ;[1 1 1] Bomb Drop
          (Development|PrintString "SCREECH!")
          (Components|Animation|PlayAnimation (Variables|Default|GetSK_Greater_Spider) "/Game/InfinityBladeAdversaries/Enemy/Enemy_Great_Spider/Enemy_SpiderGreater_Animation/ExoGame_Greater_Spider_Death.ExoGame_Greater_Spider_Death" false)
          (Utilities|FlowControl|Delay 2.0)
          (Audio|Components|Audio|Stop (Variables|Default|GetSK_Greater_Spider))
          (Effects|SpawnEmitterAttached "/Game/InfinityBladeEffects/Effects/FX_Ambient/Fog/P_ExitStair_Mist.P_ExitStair_Mist" (Variables|Default|GetParticleSystem) "None")
          (Game|SpawnActorfromClass "/Game/People/ChristianNicola/BluePrints/EggBomb.EggBomb_C" (Transformation|GetActorTransform) "Undefined" 0 0)
          (Utilities|FlowControl|Delay 5.0)
          (Actor|DestroyActor))))))

(fn ConstructionScript)