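; Greater spider enemy AI that wanders, calls for help, melees, or drops an egg bomb before destroying itself.
; BeginPlay and UpdateState run a CurrentState switch that drives animation, movement and damage, and re-enters itself to change state.
; Tick box-traces forward to set LastSeenActor, while AnyDamage sets Aggro and Enemy.
; Call for Help spawns another spider when aggroed; nothing here switches into that state or Bomb Drop.
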(event Custom|CheckSight
  ;[1 1 1] Senses
  ;;[1 1 1] Sight
  (bind (_outhit _returnvalue) (Collision|BoxTraceByChannel (Transformation|GetActorLocation) (+ (Transformation|GetActorLocation) (* (Transformation|GetActorForwardVector) 1e+04)) "100.000000,200.000000,100.000000" (Transformation|GetActorRotation) "TraceTypeQuery1" false 0 "ForOneFrame"))
  (if _returnvalue
    (Variables|Default|SetLastSeenActor (.hitactor _outhit))))

(event Custom|UpdateState
  ;[1 1 1] Random Condition
  (switch Utilities|FlowControl|Switch|SwitchonChristianNicolaStates (Variables|Default|GetCurrent%20State)
    (:NewEnumerator0
      ;[1 1 1] Wander
      (Components|Animation|PlayAnimation (Variables|Default|GetSK_Greater_Spider) "/Game/InfinityBladeAdversaries/Enemy/Enemy_Great_Spider/Enemy_SpiderGreater_Animation/ExoGame_Greater_Spider_Walk_Fwd.ExoGame_Greater_Spider_Walk_Fwd" true)
      (AI|Navigation|SimpleMovetoLocation (Pawn|GetController) (AI|Navigation|GetRandomReachablePointinRadius (Transformation|GetActorLocation) 1e+04))
      (Utilities|FlowControl|Delay (Math|Random|RandomFloatinRange 1.0 1e+01))
      (Utilities|Casting|CastToChristianAiCharacter (Variables|Default|GetLastSeenActor)
        (:then
          (CallFunction|UpdateState))
        (:CastFailed
          (Variables|Default|SetCurrent%20State "NewEnumerator3")
          (CallFunction|UpdateState))))
    (:NewEnumerator1
      ;[1 1 1] Call For Help
      (if (Variables|Default|GetAggro)
        (AI|SpawnAIFromClass "ChristianAiCharacter_C" 0 (Transformation|GetWorldLocation (Variables|Default|GetSpiderSpawnPoint1%28CallForHelp%29)) "0, 0, 0" false)
        (Timeline|Timeline_0 PlayFromStart
          (:Update
            _)
          (:Finished
            _))
        (Components|Animation|SetAnimation (Variables|Default|GetSK_Greater_Spider) "/Game/InfinityBladeAdversaries/Enemy/Enemy_Great_Spider/Enemy_SpiderGreater_Animation/ExoGame_Greater_Spider_Teleport.ExoGame_Greater_Spider_Teleport")
        (Utilities|FlowControl|Delay 5.0)
        (Audio|Components|Audio|Stop (Variables|Default|GetSK_Greater_Spider))
        (Utilities|FlowControl|Delay 2.0)
        (AI|AIMoveTo 0 "0, 0, 0" (Variables|Default|GetLastSeenActor) 5.0 false
          (:then
            _)))
      (Variables|Default|SetCurrent%20State "NewEnumerator3")
      (CallFunction|UpdateState))
    (:NewEnumerator3
      ;[1 1 1] Melee Attack
      (Utilities|IsValid (Variables|Default|GetEnemy)
        (:Is%20Valid
          (AI|Navigation|SimpleMovetoActor 0 (Variables|Default|GetEnemy))
          (Components|Animation|PlayAnimation (Variables|Default|GetSK_Greater_Spider) "/Game/InfinityBladeAdversaries/Enemy/Enemy_Great_Spider/Enemy_SpiderGreater_Animation/ExoGame_Greater_Spider_Attack_Melee.ExoGame_Greater_Spider_Attack_Melee" false)
          (Game|Damage|ApplyDamage (Variables|Default|GetLastSeenActor) 1e+02 0 self)
          (if (Game|IsActorBeingDestroyed (Variables|Default|GetLastSeenActor))
            (Variables|Default|SetCurrent%20State "NewEnumerator0")
            (CallFunction|UpdateState)
            (else
              (Variables|Default|SetCurrent%20State "NewEnumerator3")
              (CallFunction|UpdateState))))
        (:Is%20Not%20Valid
          (Variables|Default|SetCurrent%20State "NewEnumerator0")
          (CallFunction|UpdateState))))
    (:NewEnumerator4
      ;[1 1 1] Bomb Drop
      (Development|PrintString "SCREECH!")
      (Components|Animation|PlayAnimation (Variables|Default|GetSK_Greater_Spider) "/Game/InfinityBladeAdversaries/Enemy/Enemy_Great_Spider/Enemy_SpiderGreater_Animation/ExoGame_Greater_Spider_Death.ExoGame_Greater_Spider_Death" false)
      (Utilities|FlowControl|Delay 2.0)
      (Audio|Components|Audio|Stop (Variables|Default|GetSK_Greater_Spider))
      (Effects|SpawnEmitterAttached 0 0 "None")
      (Game|SpawnActorfromClass "/Game/People/ChristianNicola/BluePrints/EggBomb.EggBomb_C" (Transformation|GetActorTransform) "Undefined" 0 0)
      (Utilities|FlowControl|Delay 3.0)
      (Actor|DestroyActor))))

(event EventBeginPlay
  ;[1 1 1] Random Condition
  (switch Utilities|FlowControl|Switch|SwitchonChristianNicolaStates (Variables|Default|GetCurrent%20State)
    (:NewEnumerator0
      ;[1 1 1] Wander
      (Components|Animation|PlayAnimation (Variables|Default|GetSK_Greater_Spider) "/Game/InfinityBladeAdversaries/Enemy/Enemy_Great_Spider/Enemy_SpiderGreater_Animation/ExoGame_Greater_Spider_Walk_Fwd.ExoGame_Greater_Spider_Walk_Fwd" true)
      (AI|Navigation|SimpleMovetoLocation (Pawn|GetController) (AI|Navigation|GetRandomReachablePointinRadius (Transformation|GetActorLocation) 1e+04))
      (Utilities|FlowControl|Delay (Math|Random|RandomFloatinRange 1.0 1e+01))
      (Utilities|Casting|CastToChristianAiCharacter (Variables|Default|GetLastSeenActor)
        (:then
          (CallFunction|UpdateState))
        (:CastFailed
          (Variables|Default|SetCurrent%20State "NewEnumerator3")
          (CallFunction|UpdateState))))
    (:NewEnumerator1
      ;[1 1 1] Call For Help
      (if (Variables|Default|GetAggro)
        (AI|SpawnAIFromClass "ChristianAiCharacter_C" 0 (Transformation|GetWorldLocation (Variables|Default|GetSpiderSpawnPoint1%28CallForHelp%29)) "0, 0, 0" false)
        (Timeline|Timeline_0 PlayFromStart
          (:Update
            _)
          (:Finished
            _))
        (Components|Animation|SetAnimation (Variables|Default|GetSK_Greater_Spider) "/Game/InfinityBladeAdversaries/Enemy/Enemy_Great_Spider/Enemy_SpiderGreater_Animation/ExoGame_Greater_Spider_Teleport.ExoGame_Greater_Spider_Teleport")
        (Utilities|FlowControl|Delay 5.0)
        (Audio|Components|Audio|Stop (Variables|Default|GetSK_Greater_Spider))
        (Utilities|FlowControl|Delay 2.0)
        (AI|AIMoveTo 0 "0, 0, 0" (Variables|Default|GetLastSeenActor) 5.0 false
          (:then
            _)))
      (Variables|Default|SetCurrent%20State "NewEnumerator3")
      (CallFunction|UpdateState))
    (:NewEnumerator3
      ;[1 1 1] Melee Attack
      (Utilities|IsValid (Variables|Default|GetEnemy)
        (:Is%20Valid
          (AI|Navigation|SimpleMovetoActor 0 (Variables|Default|GetEnemy))
          (Components|Animation|PlayAnimation (Variables|Default|GetSK_Greater_Spider) "/Game/InfinityBladeAdversaries/Enemy/Enemy_Great_Spider/Enemy_SpiderGreater_Animation/ExoGame_Greater_Spider_Attack_Melee.ExoGame_Greater_Spider_Attack_Melee" false)
          (Game|Damage|ApplyDamage (Variables|Default|GetLastSeenActor) 1e+02 0 self)
          (if (Game|IsActorBeingDestroyed (Variables|Default|GetLastSeenActor))
            (Variables|Default|SetCurrent%20State "NewEnumerator0")
            (CallFunction|UpdateState)
            (else
              (Variables|Default|SetCurrent%20State "NewEnumerator3")
              (CallFunction|UpdateState))))
        (:Is%20Not%20Valid
          (Variables|Default|SetCurrent%20State "NewEnumerator0")
          (CallFunction|UpdateState))))
    (:NewEnumerator4
      ;[1 1 1] Bomb Drop
      (Development|PrintString "SCREECH!")
      (Components|Animation|PlayAnimation (Variables|Default|GetSK_Greater_Spider) "/Game/InfinityBladeAdversaries/Enemy/Enemy_Great_Spider/Enemy_SpiderGreater_Animation/ExoGame_Greater_Spider_Death.ExoGame_Greater_Spider_Death" false)
      (Utilities|FlowControl|Delay 2.0)
      (Audio|Components|Audio|Stop (Variables|Default|GetSK_Greater_Spider))
      (Effects|SpawnEmitterAttached 0 0 "None")
      (Game|SpawnActorfromClass "/Game/People/ChristianNicola/BluePrints/EggBomb.EggBomb_C" (Transformation|GetActorTransform) "Undefined" 0 0)
      (Utilities|FlowControl|Delay 3.0)
      (Actor|DestroyActor))))

(event Game|Damage|EventAnyDamage
  (params (Damage :type Float%20%28single-precision%29) (DamageType :type Damage%20Type%20Object%20Reference) (InstigatedBy :type Controller%20Object%20Reference) (DamageCauser :type Actor%20Object%20Reference))
  ;[1 1 1] Senses
  (Variables|Default|SetAggro true)
  (Variables|Default|SetEnemy InstigatedBy))

(event EventTick
  (params (DeltaSeconds :type Float%20%28single-precision%29))
  ;[1 1 1] EventTickUpdater
  (CallFunction|CheckSight))

(fn ConstructionScript)