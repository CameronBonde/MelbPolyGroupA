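; BenHumphreysBlueprint is an AI creature that wanders and celebrates when it spots another of its own kind.
; Each Tick, a forward visibility trace casts the hit actor to its own class, choosing Celebrate or Wander.
; A state switch then runs delayed actions: Wander moves to random reachable points, Celebrate jumps, and both change text and material.
; Seek, Adapt, Deploy Smoke, Attack and Explode only print their names and are never set here.
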(event Custom|UpdateState
  ;[1 1 1] Condition
  (switch Utilities|FlowControl|Switch|SwitchonBenHumphreysStates (Variables|Default|GetCurrent%20States)
    (:NewEnumerator0
      ;[1 1 1] Wander
      (Utilities|FlowControl|Delay (Math|Random|RandomFloatinRange 1.0 6.0))
      (Rendering|Components|TextRender|SetText (Variables|Default|GetTextRender) (Variables|Default|GetBeepBoopText))
      (Rendering|Material|SetMaterial (Variables|Default|GetMainSphere) 0 "/Game/People/YasmeenRooplall/Asset/wire_141007058.wire_141007058")
      (AI|Navigation|SimpleMovetoLocation (Pawn|GetController) (AI|Navigation|GetRandomReachablePointinRadius (Transformation|GetActorLocation) 1e+04))
      (Rendering|Material|SetMaterial (Variables|Default|GetMainSphere) 0 "/Game/People/YasmeenRooplall/Asset/defaultMat.defaultMat"))
    (:NewEnumerator1
      ;[1 1 1] Celebrate
      (Utilities|FlowControl|Delay 2.0)
      (Rendering|Components|TextRender|SetText (Variables|Default|GetTextRender) (Variables|Default|GetWooText))
      (Rendering|Material|SetMaterial (Variables|Default|GetMainSphere) 0 "/Game/People/YasmeenRooplall/Asset/wire_174174174.wire_174174174")
      (Character|Jump)
      (Utilities|FlowControl|Delay 0.2)
      (Development|PrintString "Woo!"))
    (:NewEnumerator6
      ;[1 1 1] Seek
      (Development|PrintString "Seek"))
    (:NewEnumerator2
      ;[1 1 1] Adapt
      (Development|PrintString "Adapt"))
    (:NewEnumerator5
      ;[1 1 1] Deploy Smoke
      (Development|PrintString "Deploy Smoke"))
    (:NewEnumerator3
      ;[1 1 1] Attack
      (Development|PrintString "Attack"))
    (:NewEnumerator4
      ;[1 1 1] Explode
      (Development|PrintString "Explode"))))

(event Custom|CheckInFront
  ;[1 1 1] Sight
  (bind _outhit (Collision|LineTraceByChannel (Transformation|GetActorLocation) (+ (Transformation|GetActorLocation) (* (Transformation|GetActorForwardVector) 1e+04)) "TraceTypeQuery1" false 0 "ForOneFrame"))
  (bind _asben_humphreys_blueprint (Utilities|Casting|CastToBenHumphreysBlueprint (.hitactor _outhit))
    (:then
      ;;[1 1 1] Saw SameSpecies, CHANGE STATE
      (Variables|Default|SetSameSpecies _asben_humphreys_blueprint)
      (Variables|Default|SetCurrent%20States "NewEnumerator1"))
    (:CastFailed
      ;;[1 1 1] Saw DifferentSpecies, CHANGE STATE
      (Variables|Default|SetCurrent%20States "NewEnumerator0"))))

(event EventTick
  (params (DeltaSeconds :type Float%20%28single-precision%29))
  ;[1 1 1] Main Loop
  (CallFunction|CheckinFront)
  (CallFunction|UpdateState))

(fn ConstructionScript)